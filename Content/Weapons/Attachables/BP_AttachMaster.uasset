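; Attachable weapon actor that resolves melee hits between the player and enemies, using the owning character's equipped weapon damage.
; BeginPlay caches the parent as player or enemy; HitDetection overlaps skip actors sharing the parent's first tag and require PlayerStats.
; Blocked hits drain stamina, play shield or sword reactions and briefly lock the attacker's attacks.
; Unblocked hits reduce health; non-lethal ones play effects and hit reactions, plus camera shake on players.
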(event OnComponentBeginOverlap(HitDetection)
  (params (OverlappedComponent :type Primitive%20Component%20Object%20Reference) (OtherActor :type Actor%20Object%20Reference) (OtherComp :type Primitive%20Component%20Object%20Reference) (OtherBodyIndex :type Integer) (bFromSweep :type Boolean) (SweepResult :type Hit%20Result%20Structure%20%28by%20ref%29))
  (Utilities|FlowControl|DelayUntilNextTick)
  (if (not (Actor|ActorHasTag OtherActor (Utilities|Array|Get(acopy) (Variables|/Script/Engine.Actor|GetTags (Actor|GetAttachParentActor)))))
    (Utilities|IsValid (Actor|GetComponentbyClass OtherActor "/Script/EnhancedTPTemplateB.PlayerStats")
      (:Is%20Valid
        (bind _asbp_base_enemy (Utilities|Casting|CastToBP_BaseEnemy OtherActor)
          (:then
            (|EnemyHitDetection _asbp_base_enemy))
          (:CastFailed
            (bind _asbp_third_person_character (Utilities|Casting|CastToBP_ThirdPersonCharacter OtherActor))
            (|PlayerHitDetection _asbp_third_person_character)))))))

(event Collision|EventActorBeginOverlap
  (params (OtherActor :type Actor%20Object%20Reference)))

(event EventBeginPlay
  (bind _returnvalue (Actor|GetAttachParentActor))
  (Utilities|FlowControl|DelayUntilNextTick)
  (Utilities|FlowControl|Sequence
    (:then_0
      (bind _asbp_third_person_character (Utilities|Casting|CastToBP_ThirdPersonCharacter _returnvalue))
      (Variables|Default|SetPlayerOwner%20Ref _asbp_third_person_character))
    (:then_1
      (bind _asbp_base_enemy (Utilities|Casting|CastToBP_BaseEnemy _returnvalue))
      (Variables|Default|SetEnemy%20Owner%20Ref _asbp_base_enemy))))

(fn ConstructionScript)