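; Base weapon pickup actor that hands its item to the player character or an enemy on overlap.
; When something enters PickupRadius, it casts to BP_ThirdPersonCharacter, then BP_BaseEnemy, and adds ItemData to that actor's InventoryComponent.
; Both successful paths share a debug print and destroy the pickup; any other actor only prints an unrecognized message.
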(event `self.PickupRadius.OnComponentBeginOverlap`
  (params (OverlappedComponent :type "PrimitiveComponent Object Reference") (OtherActor :type "Actor Object Reference") (OtherComp :type "PrimitiveComponent Object Reference") (OtherBodyIndex :type Integer) (bFromSweep :type Boolean) (SweepResult :type "HitResult Structure (by ref)"))
  (bind _itemdata_itemname (break `ItemData` (`self.ItemData`)))
  (bind _asbp_third_person_character (cast `/Game/Blueprints/BP_ThirdPersonCharacter` OtherActor)
    (:`then`
      (`InventoryComponent.AddItemToInventory` (`self.GetComponentByClass` _asbp_third_person_character "/Script/EnhancedTPTemplateB.InventoryComponent") (`self.ItemData`))
      (`KismetSystemLibrary.PrintString` (`KismetStringLibrary.Concat_StrStr` _itemdata_itemname " Added To Inventory " (`KismetSystemLibrary.GetDisplayName` _asbp_third_person_character) (`KismetSystemLibrary.GetDisplayName` (stale _asbp_base_enemy))) :!label _label)
      (`self.K2_DestroyActor`))
    (:`CastFailed`
      (bind _asbp_base_enemy (cast `/Game/Blueprints/BP_BaseEnemy` OtherActor)
        (:`then`
          (`InventoryComponent.AddItemToInventory` (`self.GetComponentByClass` _asbp_base_enemy "/Script/EnhancedTPTemplateB.InventoryComponent") (`self.ItemData`))
          (goto _label))
        (:`CastFailed`
          (`KismetSystemLibrary.PrintString` "Child Not Recognized"))))))

(fn `UserConstructionScript`)